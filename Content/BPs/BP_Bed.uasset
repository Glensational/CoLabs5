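; BP_Bed is an interactable bed that lets the player sleep to change the time of day.
; Its Box overlap adds the WB_Sleep_Prompt widget to the viewport, and leaving the box removes it.
; Interact clears the prompt, fades the camera out, sets the SunLight actor to a fixed rotation while the screen is covered, then fades back in after short delays.
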(event `/Game/BPs/BPI_Interact.Interact`
  (bind _foundwidgets (`WidgetBlueprintLibrary.GetAllWidgetsOfClass` "/Game/BPs/HUD/WB_Sleep_Prompt.WB_Sleep_Prompt_C"))
  (`Widget.RemoveFromParent` _foundwidgets)
  (`PlayerCameraManager.StartCameraFade` :`self` (`PlayerController.PlayerCameraManager` (`GameplayStatics.GetPlayerController` 0)) :`ToAlpha` 1.0 :`Duration` 1.0 :`bHoldWhenFinished` true)
  (`KismetSystemLibrary.Delay` 1.0)
  (`self.K2_SetActorRotation` (`self.SunLight`) (struct :`Yaw` -27.0 :`Roll` 455.0) false)
  (`KismetSystemLibrary.Delay` 0.5)
  (`PlayerCameraManager.StartCameraFade` :`self` (`PlayerController.PlayerCameraManager` (`GameplayStatics.GetPlayerController` 0)) :`FromAlpha` 1.0 :`Duration` 1.0 :`bHoldWhenFinished` true))

(event `self.Box.OnComponentEndOverlap`
  (params (OverlappedComponent :type "PrimitiveComponent Object Reference") (OtherActor :type "Actor Object Reference") (OtherComp :type "PrimitiveComponent Object Reference") (OtherBodyIndex :type Integer))
  (bind _foundwidgets (`WidgetBlueprintLibrary.GetAllWidgetsOfClass` "/Game/BPs/HUD/WB_Sleep_Prompt.WB_Sleep_Prompt_C"))
  (`Widget.RemoveFromParent` _foundwidgets))

(event `self.Box.OnComponentBeginOverlap`
  (params (OverlappedComponent :type "PrimitiveComponent Object Reference") (OtherActor :type "Actor Object Reference") (OtherComp :type "PrimitiveComponent Object Reference") (OtherBodyIndex :type Integer) (bFromSweep :type Boolean) (SweepResult :type "HitResult Structure (by ref)"))
  (bind _returnvalue (`|CreateWidget` "/Game/BPs/HUD/WB_Sleep_Prompt.WB_Sleep_Prompt_C"))
  (`UserWidget.AddToViewport` _returnvalue 0))

(fn `UserConstructionScript`)