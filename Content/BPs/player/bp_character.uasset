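; Player character Blueprint that handles Enhanced Input movement along world axes, creates the in-game HUD and drives a grid cursor test.
; Each tick it traces under the cursor and, on a hit, moves a cube spawned on BeginPlay to the location returned by BPCGrid, printing it for debugging.
; Interact sends a BPI_Interact message to the first overlapping actor that implements the interface.
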(event Input|EnhancedActionEvents|EnhancedInputActionIA_Move
  (params (ActionValue :type Vector%202D%20Structure) (ElapsedSeconds :type Float%20%28double-precision%29) (TriggeredSeconds :type Float%20%28double-precision%29) (InputAction :type Input%20Action%20Object%20Reference :default "/Game/Input/Actions/IA_Move.IA_Move"))
  (bind (_x _y) (Math|Vector2D|BreakVector2D ActionValue))
  ;[0.15 0.15 0.15 0.5] Character controller - Ben
  (Pawn|Input|AddMovementInput "1.000000,0.000000,0.000000" _x false)
  (Pawn|Input|AddMovementInput "0.000000,1.000000,0.000000" _y false))

(event EventBeginPlay
  ;[0.15 0.15 0.15 0.5] Character controller - Ben
  (CallFunction|CreateHUD)
  (bind _asplayer_controller (Utilities|Casting|CastToPlayerController (Pawn|GetController)))
  (Input|AddMappingContext (PlayerController|LocalPlayerSubsystems|GetEnhancedInputLocalPlayerSubsystem _asplayer_controller) "/Game/Input/IMC_Movement.IMC_Movement" 0 "(bIgnoreAllPressedKeysUntilRelease=True,bForceImmediately=False,bNotifyUserSettings=False)")
  ;[0.15 0.15 0.15 0.5] Spawns the cube so we know where the grid is for testing - Tom.
  (bind _returnvalue (Game|SpawnActorfromClass "/Game/BPs/WorldGridBP/GridCube.GridCube_C" (Math|Transform|MakeTransform "0, 0, 0" "0, 0, 0" "1.000000,1.000000,1.000000") "AlwaysSpawn" "MultiplyWithRoot" 0 0))
  (Variables|Default|SetCubeRef _returnvalue))

(event EventTick
  (params (DeltaSeconds :type Float%20%28single-precision%29))
  (bind _bpc_grid (Variables|Default|GetBPC_Grid))
  (bind _cursorlocation (Variables|Default|GetCursorLocation))
  (bind _locationongrid (Default|GetGridLocation _bpc_grid _cursorlocation))
  ;[0.15 0.15 0.15 0.5] This finds the location of the cursor and divides the world into a grid using the GetCursorLocation function - Tom.
  (CallFunction|GetCursorLocation)
  (if (Variables|Default|GetCursorHit)
    (Development|PrintString (Utilities|String|ToString(Vector) _locationongrid) true true "(R=0.000000,G=0.660000,B=1.000000,A=1.000000)" 0.0)
    (Transformation|SetWorldLocation (Variables|/Script/Engine.Actor|GetRootComponent (Variables|Default|GetCubeRef)) _locationongrid false false)))

(event Input|ActionEvents|InputActionInteract
  (params (Key :type Key%20Structure :default "None"))
  ;[0.15 0.15 0.15 0.5] Interact System - Luke
  (:Pressed
    (bind _array_element (Utilities|Array|ForEachLoopwithBreak (Collision|GetOverlappingActors "/Script/Engine.Actor" :!class /Script/Engine.Actor) :!label _label)
      (:LoopBody
        (if (Utilities|DoesObjectImplementInterface _array_element "/Game/BPs/BPI_Interact.BPI_Interact_C")
          (Class|BPIInteract|Interact(Message) _array_element)
          (goto _label Break))))))

(fn ConstructionScript)

(fn GetCursorLocation
  (bind _returnvalue (Game|GetPlayerController 0))
  (bind _hitresult (Game|Player|GetHitResultUnderCursorbyChannel _returnvalue "TraceTypeQuery1" true))
  (bind (_bblockinghit _binitialoverlap _time _distance _location) (Collision|BreakHitResult _hitresult))
  ;[0.15 0.15 0.15 0.5] Converts Hit Results to Cursor Location for Grid Script - Tom.
  (Variables|Default|SetCursorHit _bblockinghit)
  (Variables|Default|SetCursorLocation _location)
  (return))

(fn CreateHUD
  ;[0.15 0.15 0.15 0.5] Creates HUD in separate area.
  (bind _returnvalue (UserInterface|CreateWidget "/Game/BPs/HUD/PlayerHUDInGame.PlayerHUDInGame_C"))
  (UserInterface|Viewport|AddtoViewport _returnvalue 0)
  (return))